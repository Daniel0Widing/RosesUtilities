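; BP_Packager is a placeable container structure that can be switched on and off, with visual effects for its active state.
; Activation disables structure pickup, sets the activate prompt to "Turn On" and shows the goo, gas and electrical arc components.
; Deactivation only hides those components, and no packaging logic appears in these graphs.
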(fn ConstructionScript)

(fn BPContainerActivated
  (Class|PrimalStructure|DisableStructurePickup)
  (Variables|Default|SetActivateContainerString "Turn On")
  (Rendering|SetVisibility (Variables|Default|GetGoo1) true false))

(fn BPContainerDeactivated
  (Rendering|SetVisibility (Variables|Default|GetGoo1) false false))