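; BP_DinoDaycare is a placeable structure that automatically claims, feeds and imprints baby dinos within a configurable range.
; BeginPlay reads range, claim and fuel-consumption settings from the global utilities actor, then starts a looping server-side octree scan that unstasises babies.
; Unclaimed babies join the owning team when the multi-use toggle allows it.
; Team babies get food and age-scaled imprint credited to the placing player, with imprinting requiring activation unless fuel consumption is zero.
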(event EventBeginPlay
  (|CallParentFunction)
  (if (not (Variables|Default|GetbIsPreviewStructure))
    ;[1 1 1] Gets effect range config and claiming enabled config
    (bind _globalactor (CallFunction|RUGetGlobalActor self))
    (Variables|Default|SeteffectRange (* (Variables|/Game/Mods/RosesUtilities/RosesUtilities_GlobalActor.RosesUtilities_GlobalActor_C|GetDinoDaycareRange _globalactor) 3e+02) false)
    (Variables|Default|SetisClaimingEnabledInConfig (Variables|/Game/Mods/RosesUtilities/RosesUtilities_GlobalActor.RosesUtilities_GlobalActor_C|GetDinoDaycareAllowAutoClaim _globalactor) false)
    (if (Variables|/Game/Mods/RosesUtilities/RosesUtilities_GlobalActor.RosesUtilities_GlobalActor_C|GetDinoDaycareAllowAutoClaim _globalactor)
      _
      (else
        (Variables|Default|SetisClaimingActive false false)))
    ;[1 1 1] Disables rare flower use if config is 0, otherwise sets consumption to config
    (if (== (Variables|/Game/Mods/RosesUtilities/RosesUtilities_GlobalActor.RosesUtilities_GlobalActor_C|GetDinoDaycareConsumptionRate _globalactor) 0.0)
      (Variables|Default|SetbCanToggleActivation false)
      (Variables|Default|SetisImprintingForceAllowed true)
      (else
        (Variables|Default|SetFuelConsumptionIntervalsMultiplier (/ 1.0 (Variables|/Game/Mods/RosesUtilities/RosesUtilities_GlobalActor.RosesUtilities_GlobalActor_C|GetDinoDaycareConsumptionRate _globalactor)))))
    (Utilities|FlowControl|Delay 0.7)
    (Utilities|Time|SetTimerbyFunctionName 0 "HandleNearbyBabies" 1e+01 true)))

(fn ConstructionScript
  (|CallParentFunction))

(fn HandleNearbyBabies
  (bind _placementshootercharacter (Variables|Default|GetplacementShooterCharacter))
  (bind _placementshootercharacter_2 (Variables|Default|GetplacementShooterCharacter))
  (bind _lastvalidplayercontroller (Variables|/Script/ShooterGame.ShooterCharacter|GetLastValidPlayerController _placementshootercharacter_2))
  (Class|KismetSystemLibrary|IsRunningonServer
    (:Yes
      ;[1 1 1] Disables if range is 0
      (if (> (Variables|Default|GeteffectRange) 0.0)
        (bind _returnvalue (Class|VictoryCore|ServerOctreeOverlapActorsClass (Class|Actor|GetWorld) (Transformation|GetActorLocation) (Variables|Default|GeteffectRange) "DINOPAWNS" "/Script/ShooterGame.PrimalDinoCharacter" true))
        (for _array_element _returnvalue
          (bind _asprimaldinocharacter (Utilities|Casting|CastToPrimalDinoCharacter _array_element))
          (if (Variables|/Script/ShooterGame.PrimalDinoCharacter|GetbIsBaby _asprimaldinocharacter)
            (LocalVariables|SettempDino _asprimaldinocharacter)
            (Utilities|FlowControl|Sequence
              (:then_0
                ;[1 1 1] Unstasises baby dino to handle it
                (if (Variables|/Script/Engine.Actor|GetbStasised (LocalVariables|GettempDino))
                  (Class|Actor|Unstasis (LocalVariables|GettempDino))
                  (Class|PrimalInventoryComponent|InventoryRefresh (Variables|/Script/ShooterGame.PrimalCharacter|GetMyInventoryComponent (LocalVariables|GettempDino)))))
              (:then_1
                ;[1 1 1] Auto claims the dino if valid
                (if (and (== (Variables|/Script/Engine.Actor|GetTargetingTeam (LocalVariables|GettempDino)) 2000000000) (Variables|Default|GetisClaimingActive))
                  (Variables|/Script/Engine.Actor|SetTargetingTeam (LocalVariables|GettempDino) (Variables|Default|GetTargetingTeam) false)
                  (Class|PrimalDinoCharacter|BPNotifyClaimed (LocalVariables|GettempDino))))
              (:then_2
                ;[1 1 1] Auto feeds the dino if valid
                (if (and (<= (Variables|/Script/ShooterGame.PrimalDinoCharacter|GetBabyAge (LocalVariables|GettempDino)) 0.99) (== (Variables|/Script/Engine.Actor|GetTargetingTeam (LocalVariables|GettempDino)) (Variables|Default|GetTargetingTeam)))
                  (Class|PrimalCharacterStatusComponent|AddStatusValueModifier (Variables|/Script/ShooterGame.PrimalCharacter|GetMyCharacterStatusComponent (LocalVariables|GettempDino)) "Food" (* (Math|Conversions|ToFloat(Integer) (Class|PrimalCharacterStatusComponent|GetStatusMaxValueString (Variables|/Script/ShooterGame.PrimalCharacter|GetMyCharacterStatusComponent (LocalVariables|GettempDino)) "Food" true)) (+ (Variables|/Script/ShooterGame.PrimalDinoCharacter|GetBabyAge (LocalVariables|GettempDino)) 0.1)) 0.0 false true 0 false 0.0 false "MAX" false)))
              (:then_3
                ;[1 1 1] Auto imprints the dino by percent if valid
                (if (and (== (Variables|/Script/Engine.Actor|GetTargetingTeam (LocalVariables|GettempDino)) (Variables|Default|GetTargetingTeam)) (or (Variables|Default|GetbContainerActivated) (Variables|Default|GetisImprintingForceAllowed)))
                  (Utilities|FlowControl|Sequence
                    (:then_0
                      (Utilities|IsValid _placementshootercharacter
                        (:Is%20Valid
                          (Class|PrimalDinoCharacter|SetImprintPlayer (LocalVariables|GettempDino) _placementshootercharacter)
                          (Utilities|IsValid _lastvalidplayercontroller
                            (:Is%20Valid
                              (Class|PrimalDinoCharacter|UpdateImprintingDetailsforController (LocalVariables|GettempDino) _lastvalidplayercontroller))))))
                    (:then_1
                      (Class|PrimalDinoCharacter|UpdateImprintingQuality (LocalVariables|GettempDino) (Math|Float|Min(Float) (Math|Float|Max(Float) (+ (Variables|/Script/ShooterGame.PrimalDinoCharacter|GetBabyAge (LocalVariables|GettempDino)) 0.1) (Variables|/Script/ShooterGame.PrimalCharacterStatusComponent|GetDinoImprintingQuality (Variables|/Script/ShooterGame.PrimalCharacter|GetMyCharacterStatusComponent (LocalVariables|GettempDino)))) 1.0))
                      (Class|PrimalCharacterStatusComponent|RescaleAllStats (Variables|/Script/ShooterGame.PrimalCharacter|GetMyCharacterStatusComponent (LocalVariables|GettempDino)))
                      (Class|PrimalCharacterStatusComponent|ServerSyncReplicatedValues (Variables|/Script/ShooterGame.PrimalCharacter|GetMyCharacterStatusComponent (LocalVariables|GettempDino))))))))))))))

(fn BPTryMultiUse
  (params (ForPC :type Player%20Controller%20Object%20Reference) (UseIndex :type Integer))
  (|CallParentFunction ForPC UseIndex)
  (Utilities|FlowControl|Sequence
    (:then_0
      (switch string (Utilities|String|ToString(Integer) UseIndex)
        (:90314
          ;[1 1 1] Toggles if auto claim is active
          (Variables|Default|SetisClaimingActive (not (Variables|Default|GetisClaimingActive)) true))))
    (:then_1
      (return true))))

(fn BPGetMultiUseEntries
  (params (ForPC :type Player%20Controller%20Object%20Reference) (MultiUseEntries :type Array%20of%20Multi%20Use%20Entry%20Structures))
  (bind _returnvalue (|CallParentFunction ForPC MultiUseEntries))
  (LocalVariables|SettempMultiUseEntries _returnvalue)
  (if (== (Variables|Default|GetTargetingTeam) (Variables|/Script/Engine.Actor|GetTargetingTeam ForPC))
    (Utilities|FlowControl|Sequence
      (:then_0
        ;[1 1 1] Adds a MultiUse entry to toggle auto claiming babies on or off
        (if (Variables|Default|GetisClaimingEnabledInConfig)
          (Utilities|Array|Add (LocalVariables|GettempMultiUseEntries) (Utilities|Struct|MakeMultiUseEntry 0 (Utilities|String|SelectString "Disable Auto-Claim Babies" "Enable Auto-Claim Babies" (Variables|Default|GetisClaimingActive)) 90314 -10000))))
      (:then_1
        (return (LocalVariables|GettempMultiUseEntries))))
    (else
      (return (LocalVariables|GettempMultiUseEntries)))))

(fn BPPlacedStructure
  (params (ForPC :type Player%20Controller%20Object%20Reference))
  (Variables|Default|SetplacementShooterCharacter (Class|VictoryCore|GetShooterCharacterfromController ForPC)))