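; Industrial composter structure that automatically collects dropped feces and distributes compost fertilizer to nearby same-team crop plots.
; Looping timers drive server-only octree searches within a radius scaled from the global actor's config, with zero disabling both features.
; Collection pulls whitelisted same-team drops into its inventory, while distribution feeds plots that are low on fertilizer and have free slots.
; Same-team players toggle each feature through multi-use menu entries.
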(event EventBeginPlay
  (|CallParentFunction)
  (if (not (Variables|Default|GetbIsPreviewStructure))
    ;[1 1 1] Gets auto-collect/distribute range config
    (bind _globalactor (CallFunction|RUGetGlobalActor self))
    (Variables|Default|SeteffectRange (* 300 (Variables|/Game/Mods/RosesUtilities/RosesUtilities_GlobalActor.RosesUtilities_GlobalActor_C|GetIndustrialComposterRange _globalactor)) true)
    (Utilities|FlowControl|Delay 0.3)
    (Utilities|Time|SetTimerbyFunctionName 0 "AutoCollectItems" 1e+01 true)
    (Utilities|Time|SetTimerbyFunctionName 0 "AutoDistributeItems" 1e+01 true)))

(fn ConstructionScript
  (|CallParentFunction))

(fn BPGetMultiUseEntries
  (params (ForPC :type Player%20Controller%20Object%20Reference) (MultiUseEntries :type Array%20of%20Multi%20Use%20Entry%20Structures))
  (bind _returnvalue (|CallParentFunction ForPC MultiUseEntries))
  (LocalVariables|SettempMultiUseEntries _returnvalue)
  (if (== (Variables|Default|GetTargetingTeam) (Variables|/Script/Engine.Actor|GetTargetingTeam ForPC))
    (Utilities|FlowControl|Sequence
      (:then_0
        ;[1 1 1] Adds a MultiUse entry to toggle particles on or off
        (Utilities|Array|Add (LocalVariables|GettempMultiUseEntries) (Utilities|Struct|MakeMultiUseEntry 0 (Utilities|String|SelectString "Disable Auto-Distribute" "Enable Auto-Distribute" (Variables|Default|GetisAutoDistributeActive)) 90314 -10000)))
      (:then_1
        ;[1 1 1] Adds a MultiUse entry to toggle auto-collect on or off
        (Utilities|Array|Add (LocalVariables|GettempMultiUseEntries) (Utilities|Struct|MakeMultiUseEntry 0 (Utilities|String|SelectString "Disable Auto-Collect" "Enable Auto-Collect" (Variables|Default|GetisAutoCollectActive)) 90414 -10001)))
      (:then_2
        (return (LocalVariables|GettempMultiUseEntries))))
    (else
      (return (LocalVariables|GettempMultiUseEntries)))))

(fn BPTryMultiUse
  (params (ForPC :type Player%20Controller%20Object%20Reference) (UseIndex :type Integer))
  (|CallParentFunction ForPC UseIndex)
  (Utilities|FlowControl|Sequence
    (:then_0
      (switch string (Utilities|String|ToString(Integer) UseIndex)
        (:90314
          ;[1 1 1] Toggles auto-distribute
          (Variables|Default|SetisAutoDistributeActive (not (Variables|Default|GetisAutoDistributeActive)) true))
        (:90414
          ;[1 1 1] Toggles auto-collect
          (Variables|Default|SetisAutoCollectActive (not (Variables|Default|GetisAutoCollectActive)) true))))
    (:then_1
      (return true))))

(fn AutoCollectItems
  (Class|KismetSystemLibrary|IsRunningonServer
    (:Yes
      ;[1 1 1] Disables if range is 0
      (if (> (Variables|Default|GeteffectRange) 0.0)
        ;[1 1 1] Gets all dropped items in range
        (if (Variables|Default|GetisAutoCollectActive)
          (bind _returnvalue (Class|VictoryCore|ServerOctreeOverlapActorsClass (Class|Actor|GetWorld) (Transformation|GetActorLocation) (Variables|Default|GeteffectRange) "ALL_SPATIAL" "/Script/ShooterGame.DroppedItem" true))
          ;[1 1 1] Picks up each dropped feces in range, stops if inventory is full
          (for _array_element _returnvalue
            (if (== (Variables|/Script/Engine.Actor|GetTargetingTeam _array_element) (Variables|Default|GetTargetingTeam))
              (CallFunction|RUPickupItemtoInventory _array_element (Variables|Default|GetMyInventoryComponent) (Utilities|Array|MakeArray "/Game/PrimalEarth/CoreBlueprints/Items/Consumables/BaseBPs/PrimalItemConsumablePoop.PrimalItemConsumablePoop_C")))))))))

(fn AutoDistributeItems
  (Class|KismetSystemLibrary|IsRunningonServer
    (:Yes
      ;[1 1 1] Disables if range is 0
      (if (> (Variables|Default|GeteffectRange) 0.0)
        ;[1 1 1] Checks distribute is active and inventory has fertilizer to distribute
        (if (Variables|Default|GetisAutoDistributeActive)
          (bind _returnvalue (Class|PrimalInventoryComponent|GetItemTemplateQuantity (Variables|Default|GetMyInventoryComponent) "/Game/PrimalEarth/CoreBlueprints/Items/Consumables/BaseBPs/PrimalItemConsumable_Fertilizer_Base.PrimalItemConsumable_Fertilizer_Base_C" 0 true false false false))
          (if (> _returnvalue 0)
            ;[1 1 1] Gets all crop plots in range
            (bind _returnvalue_2 (Class|VictoryCore|ServerOctreeOverlapActorsClass (Class|Actor|GetWorld) (Transformation|GetActorLocation) (Variables|Default|GeteffectRange) "STRUCTURES" "/Game/PrimalEarth/Structures/BuildingBases/CropPlotBaseBP.CropPlotBaseBP_C" true))
            ;[1 1 1] Distributes to crop plots of the same team and with less than 2 fertilizer in them and room in their inventory
            (for _array_element _returnvalue_2
              (bind _ascropplotbasebp_c (Utilities|Casting|CastToCropPlotBaseBP _array_element))
              (if (== (Variables|/Script/Engine.Actor|GetTargetingTeam _ascropplotbasebp_c) (Variables|Default|GetTargetingTeam))
                (bind _returnvalue_3 (Class|PrimalInventoryComponent|GetItemTemplateQuantity (Variables|/Script/ShooterGame.PrimalStructureItemContainer|GetMyInventoryComponent _ascropplotbasebp_c) "/Game/PrimalEarth/CoreBlueprints/Items/Consumables/BaseBPs/PrimalItemConsumable_Fertilizer_Base.PrimalItemConsumable_Fertilizer_Base_C" 0 true false false false))
                (bind _hasemptyslots (CallFunction|RUDoesInventoryHaveEmptySlots (Variables|/Script/ShooterGame.PrimalStructureItemContainer|GetMyInventoryComponent _ascropplotbasebp_c)))
                (if (and _hasemptyslots (< _returnvalue_3 2))
                  (CallFunction|RUTransferFirstItemOfClassfromInventory (Variables|Default|GetMyInventoryComponent) (Variables|/Script/ShooterGame.PrimalStructureItemContainer|GetMyInventoryComponent _ascropplotbasebp_c) "/Game/PrimalEarth/CoreBlueprints/Items/Consumables/PrimalItemConsumable_Fertilizer_Compost.PrimalItemConsumable_Fertilizer_Compost_C" true false false false))))))))))