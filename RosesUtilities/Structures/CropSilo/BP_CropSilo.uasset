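; Crop silo storage structure that automatically collects vegetables from nearby crop plots on the same team.
; A looping server-effective timer runs an octree overlap within a radius scaled by the global config actor, transferring matching items into the silo; zero range disables it.
; A team-only multi-use entry toggles auto-collect.
; Inventory changes update HasInventory, whose OnRep shows or hides the crop meshes.
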(event EventBeginPlay
  (|CallParentFunction)
  (if (not (Variables|Default|GetbIsPreviewStructure))
    ;[1 1 1] Gets auto-collect range config
    (bind _globalactor (CallFunction|RUGetGlobalActor self))
    (Variables|Default|SeteffectRange (* 300 (Variables|/Game/Mods/RosesUtilities/RosesUtilities_GlobalActor.RosesUtilities_GlobalActor_C|GetCropSiloAutoCollectRange _globalactor)) true)
    (Utilities|FlowControl|Delay 0.4)
    (Utilities|Time|SetTimerbyFunctionName 0 "AutoCollectItems" 1e+01 true)))

(fn ConstructionScript
  (|CallParentFunction))

(fn BPNotifyInventoryItemChange
  (params (bIsItemAdd :type Boolean) (theItem :type Primal%20Item%20Object%20Reference) (bEquipItem :type Boolean))
  (Variables|Default|SethasInventory (> (Utilities|Array|Length (Variables|/Script/ShooterGame.PrimalInventoryComponent|GetInventoryItems (Variables|Default|GetMyInventoryComponent))) 0) true))

(fn BPGetMultiUseEntries
  (params (ForPC :type Player%20Controller%20Object%20Reference) (MultiUseEntries :type Array%20of%20Multi%20Use%20Entry%20Structures))
  (bind _returnvalue (|CallParentFunction ForPC MultiUseEntries))
  (LocalVariables|SettempMultiUseEntries _returnvalue)
  (if (== (Variables|Default|GetTargetingTeam) (Variables|/Script/Engine.Actor|GetTargetingTeam ForPC))
    (Utilities|FlowControl|Sequence
      (:then_0
        ;[1 1 1] Adds a MultiUse entry to toggle auto-collect on or off
        (Utilities|Array|Add (LocalVariables|GettempMultiUseEntries) (Utilities|Struct|MakeMultiUseEntry 0 (Utilities|String|SelectString "Disable Auto-Collect" "Enable Auto-Collect" (Variables|Default|GetisAutoCollectActive)) 90414 -10001)))
      (:then_1
        (return (LocalVariables|GettempMultiUseEntries))))
    (else
      (return (LocalVariables|GettempMultiUseEntries)))))

(fn BPTryMultiUse
  (params (ForPC :type Player%20Controller%20Object%20Reference) (UseIndex :type Integer))
  (|CallParentFunction ForPC UseIndex)
  (Utilities|FlowControl|Sequence
    (:then_0
      (switch string (Utilities|String|ToString(Integer) UseIndex)
        (:90414
          ;[1 1 1] Toggles auto-collect
          (Variables|Default|SetisAutoCollectActive (not (Variables|Default|GetisAutoCollectActive)) true))))
    (:then_1
      (return true))))

(fn AutoCollectItems
  (Class|KismetSystemLibrary|IsRunningonServer
    (:Yes
      ;[1 1 1] Disables if range is 0
      (if (> (Variables|Default|GeteffectRange) 0.0)
        (if (Variables|Default|GetisAutoCollectActive)
          (bind _returnvalue (Class|VictoryCore|ServerOctreeOverlapActorsClass (Class|Actor|GetWorld) (Transformation|GetActorLocation) (Variables|Default|GeteffectRange) "STRUCTURES" "/Game/PrimalEarth/Structures/BuildingBases/CropPlotBaseBP.CropPlotBaseBP_C" true))
          (for _array_element _returnvalue
            (if (== (Variables|/Script/Engine.Actor|GetTargetingTeam _array_element) (Variables|Default|GetTargetingTeam))
              (bind _asprimalstructureitemcontainer (Utilities|Casting|CastToPrimalStructureItemContainer _array_element))
              (CallFunction|RUTransferAllItems (Variables|/Script/ShooterGame.PrimalStructureItemContainer|GetMyInventoryComponent _asprimalstructureitemcontainer) (Variables|Default|GetMyInventoryComponent) (Utilities|Array|MakeArray "/Game/PrimalEarth/CoreBlueprints/Items/Consumables/BaseBPs/PrimalItemConsumable_Veggie_Base.PrimalItemConsumable_Veggie_Base_C") false true false false false))))))))

(fn OnRepHasInventory
  (Rendering|SetVisibility (Variables|Default|GetCropMeshes) (Variables|Default|GethasInventory) true))