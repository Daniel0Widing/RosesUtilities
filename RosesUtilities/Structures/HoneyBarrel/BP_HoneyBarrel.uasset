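; BP_HoneyBarrel is a honey barrel structure that shows honey and bee effects only while its inventory holds items.
; Inventory change notifications set a HasInventory flag from whether the honey barrel inventory component contains any items.
; A throttled tick compares that flag to the Bees component's visibility and, on a mismatch, toggles the bees and all honey components together.
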(fn ConstructionScript
  (|CallParentFunction))

(fn BPNotifyInventoryItemChange
  (params (bIsItemAdd :type Boolean) (theItem :type Primal%20Item%20Object%20Reference) (bEquipItem :type Boolean))
  (Variables|Default|SetHasInventory (> (Utilities|Array|Length (Variables|/Script/ShooterGame.PrimalInventoryComponent|GetInventoryItems (Variables|Default|GetPrimalInventoryBP_HoneyBarrel_C1))) 0) true))

(fn ThrottledTick
  (bind _hasinventory (Variables|Default|GetHasInventory))
  ;[1 1 1] Toggles SFX based on if structure has inventory
  (if (not (Math|Boolean|Equal(Boolean) (Variables|/Script/Engine.SceneComponent|GetbVisible (Variables|Default|GetBees)) _hasinventory))
    (Rendering|SetVisibility (Variables|Default|GetHoney) _hasinventory false)))