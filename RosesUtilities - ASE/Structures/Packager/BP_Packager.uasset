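; Packager item-container structure that auto-collects allowed items from nearby same-team dinos and whitelisted structures.
; A looping server timer runs an octree overlap within a config-driven range, transferring items matching its inventory's allowed classes, minus the first entry.
; Wood types are excluded from structure pulls to preserve forge fuel.
; Team-only multi-use toggles collection and lengthens the pickup hold while activated; replicated activation state drives particle visibility.
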(event EventParentFirstBeginPlay
  (Utilities|FlowControl|Sequence
    (:then_0
      ;[1 1 1] Gets auto-collect range config
      (Class|KismetSystemLibrary|IsRunningonServer
        (:Yes
          (bind _globalactor (CallFunction|RUGetGlobalActor self))
          (Variables|Default|SeteffectRange (* 300 (Variables|/Game/Mods/RosesUtilities/RosesUtilities_GlobalActor.RosesUtilities_GlobalActor_C|GetPackagerAutoCollectRange _globalactor)) true))))
    (:then_1
      ;[1 1 1] Restores saved visibility
      (CallFunction|OnRepEffectRange)
      (CallFunction|OnRepIsActivated))
    (:then_2
      ;[1 1 1] Starts item collect scan loop
      (Class|KismetSystemLibrary|IsRunningonServer
        (:Yes
          (Utilities|FlowControl|Delay 0.1)
          (Utilities|Time|SetTimerbyFunctionName 0 "AutoCollectItems" 1e+01 true))))))

(fn ConstructionScript)

(fn BPContainerActivated
  (Variables|Default|SetisActivated true true)
  (if (not (Variables|Default|GethasBeenActivated))
    (Variables|Default|SethasBeenActivated true true)))

(fn BPTryMultiUse
  (params (ForPC :type Player%20Controller%20Object%20Reference) (UseIndex :type Integer))
  (|CallParentFunction ForPC UseIndex)
  (Utilities|FlowControl|Sequence
    (:then_0
      (switch string (Utilities|String|ToString(Integer) UseIndex)
        (:90414
          ;[1 1 1] Toggles auto-collect
          (Variables|Default|SetisAutoCollectActive (not (Variables|Default|GetisAutoCollectActive)) true))))
    (:then_1
      (return true))))

(fn BPGetMultiUseEntries
  (params (ForPC :type Player%20Controller%20Object%20Reference) (MultiUseEntries :type Array%20of%20Multi%20Use%20Entry%20Structures))
  (bind _returnvalue (|CallParentFunction ForPC MultiUseEntries))
  (LocalVariables|SettempMultiUseEntries _returnvalue)
  (if (== (Variables|Default|GetTargetingTeam) (Variables|/Script/Engine.Actor|GetTargetingTeam ForPC))
    (Utilities|FlowControl|Sequence
      (:then_0
        (if (Variables|Default|GetbContainerActivated)
          ;[1 1 1] Extends Pickup multiuse activation timer
          (bind (_array_element _array_index) (Utilities|Array|ForEachLoopwithBreak (LocalVariables|GettempMultiUseEntries) :!label _label)
            (:LoopBody
              (if (== (.UseIndex (Utilities|Struct|BreakMultiUseEntry _array_element)) 203)
                (Utilities|Array|SetArrayElem (LocalVariables|GettempMultiUseEntries) _array_index (Utilities|Struct|MakeMultiUseEntry (.ForComponent (Utilities|Struct|BreakMultiUseEntry (Utilities|Array|Get(acopy) (LocalVariables|GettempMultiUseEntries) _array_index))) (.UseString (Utilities|Struct|BreakMultiUseEntry (Utilities|Array|Get(acopy) (LocalVariables|GettempMultiUseEntries) _array_index))) (.UseIndex (Utilities|Struct|BreakMultiUseEntry (Utilities|Array|Get(acopy) (LocalVariables|GettempMultiUseEntries) _array_index))) (.Priority (Utilities|Struct|BreakMultiUseEntry (Utilities|Array|Get(acopy) (LocalVariables|GettempMultiUseEntries) _array_index))) (.bHideFromUI (Utilities|Struct|BreakMultiUseEntry (Utilities|Array|Get(acopy) (LocalVariables|GettempMultiUseEntries) _array_index))) (.bDisableUse (Utilities|Struct|BreakMultiUseEntry (Utilities|Array|Get(acopy) (LocalVariables|GettempMultiUseEntries) _array_index))) (.bHideActivationKey (Utilities|Struct|BreakMultiUseEntry (Utilities|Array|Get(acopy) (LocalVariables|GettempMultiUseEntries) _array_index))) (.bRepeatMultiUse (Utilities|Struct|BreakMultiUseEntry (Utilities|Array|Get(acopy) (LocalVariables|GettempMultiUseEntries) _array_index))) (.bDisplayOnInventoryUI (Utilities|Struct|BreakMultiUseEntry (Utilities|Array|Get(acopy) (LocalVariables|GettempMultiUseEntries) _array_index))) (.bDisplayOnInventoryUISecondary (Utilities|Struct|BreakMultiUseEntry (Utilities|Array|Get(acopy) (LocalVariables|GettempMultiUseEntries) _array_index))) (.bHarvestable (Utilities|Struct|BreakMultiUseEntry (Utilities|Array|Get(acopy) (LocalVariables|GettempMultiUseEntries) _array_index))) (.bIsSecondaryUse (Utilities|Struct|BreakMultiUseEntry (Utilities|Array|Get(acopy) (LocalVariables|GettempMultiUseEntries) _array_index))) (.bPersistWheelOnActivation (Utilities|Struct|BreakMultiUseEntry (Utilities|Array|Get(acopy) (LocalVariables|GettempMultiUseEntries) _array_index))) (.bOverrideUseTextColor (Utilities|Struct|BreakMultiUseEntry (Utilities|Array|Get(acopy) (LocalVariables|GettempMultiUseEntries) _array_index))) (.bDisplayOnInventoryUITertiary (Utilities|Struct|BreakMultiUseEntry (Utilities|Array|Get(acopy) (LocalVariables|GettempMultiUseEntries) _array_index))) (.bClientSideOnly (Utilities|Struct|BreakMultiUseEntry (Utilities|Array|Get(acopy) (LocalVariables|GettempMultiUseEntries) _array_index))) (.bPersistWheelRequiresDirectActivation (Utilities|Struct|BreakMultiUseEntry (Utilities|Array|Get(acopy) (LocalVariables|GettempMultiUseEntries) _array_index))) (.bDrawTooltip (Utilities|Struct|BreakMultiUseEntry (Utilities|Array|Get(acopy) (LocalVariables|GettempMultiUseEntries) _array_index))) (.WheelCategory (Utilities|Struct|BreakMultiUseEntry (Utilities|Array|Get(acopy) (LocalVariables|GettempMultiUseEntries) _array_index))) (.DisableUseColor (Utilities|Struct|BreakMultiUseEntry (Utilities|Array|Get(acopy) (LocalVariables|GettempMultiUseEntries) _array_index))) (.UseTextColor (Utilities|Struct|BreakMultiUseEntry (Utilities|Array|Get(acopy) (LocalVariables|GettempMultiUseEntries) _array_index))) 3e+01 3e+01 (.ActivationSound (Utilities|Struct|BreakMultiUseEntry (Utilities|Array|Get(acopy) (LocalVariables|GettempMultiUseEntries) _array_index))) (.UseInventoryButtonStyleOverrideIndex (Utilities|Struct|BreakMultiUseEntry (Utilities|Array|Get(acopy) (LocalVariables|GettempMultiUseEntries) _array_index))) (.AdditionalButtonsIndex (Utilities|Struct|BreakMultiUseEntry (Utilities|Array|Get(acopy) (LocalVariables|GettempMultiUseEntries) _array_index)))))
                (goto _label Break))))))
      (:then_1
        ;[1 1 1] Adds a MultiUse entry to toggle auto-collect on or off
        (Utilities|Array|Add (LocalVariables|GettempMultiUseEntries) (Utilities|Struct|MakeMultiUseEntry 0 (Utilities|String|SelectString "Disable Auto-Collect" "Enable Auto-Collect" (Variables|Default|GetisAutoCollectActive)) 90414 -10001)))
      (:then_2
        (return (LocalVariables|GettempMultiUseEntries))))
    (else
      (return (LocalVariables|GettempMultiUseEntries)))))

(fn AutoCollectItems
  (Class|KismetSystemLibrary|IsRunningonServer
    (:Yes
      ;[1 1 1] Disables if range is 0
      (if (> (Variables|Default|GeteffectRange) 0.0)
        (if (Variables|Default|GetisAutoCollectActive)
          ;[1 1 1] Gets items allowed to be collected from the items that can be inserted into the inventory, wood is excluded from structures for forge fuel
          (LocalVariables|SetitemsToCollect (Variables|/Script/ShooterGame.PrimalInventoryComponent|GetRemoteAddItemOnlyAllowItemClasses (Variables|Default|GetPrimalInventoryBP_Packager_C1)))
          (Utilities|Array|RemoveIndex (LocalVariables|GetitemsToCollect))
          (LocalVariables|SetitemsToCollect_Structures (LocalVariables|GetitemsToCollect))
          (Utilities|Array|RemoveItem (LocalVariables|GetitemsToCollect_Structures) "/Game/PrimalEarth/CoreBlueprints/Resources/PrimalItemResource_Wood.PrimalItemResource_Wood_C")
          (Utilities|Array|RemoveItem (LocalVariables|GetitemsToCollect_Structures) "/Game/Aberration/CoreBlueprints/Resources/PrimalItemResource_FungalWood.PrimalItemResource_FungalWood_C")
          (Utilities|Array|RemoveItem (LocalVariables|GetitemsToCollect_Structures) "/Game/Extinction/CoreBlueprints/Resources/PrimalItemResource_CorruptedWood.PrimalItemResource_CorruptedWood_C")
          (bind _returnvalue (Class|VictoryCore|ServerOctreeOverlapActors (Class|Actor|GetWorld) (Transformation|GetActorLocation) (Variables|Default|GeteffectRange) "TARGETABLEACTORS" true))
          (for _array_element _returnvalue
            (if (== (Variables|/Script/Engine.Actor|GetTargetingTeam _array_element) (Variables|Default|GetTargetingTeam))
              (Utilities|FlowControl|Sequence
                (:then_0
                  (bind _asprimalstructureitemcontainer (Utilities|Casting|CastToPrimalStructureItemContainer _array_element))
                  (bind _globalactor (CallFunction|RUGetGlobalActor _asprimalstructureitemcontainer))
                  (if (Utilities|Array|ContainsItem (Variables|/Game/Mods/RosesUtilities/RosesUtilities_GlobalActor.RosesUtilities_GlobalActor_C|GetPackagerAutoCollectStructureWhitelist _globalactor) (Utilities|GetClassDisplayName (Utilities|GetClass _asprimalstructureitemcontainer)))
                    (CallFunction|RUTransferAllItems (Variables|/Script/ShooterGame.PrimalStructureItemContainer|GetMyInventoryComponent _asprimalstructureitemcontainer) (Variables|Default|GetMyInventoryComponent) (LocalVariables|GetitemsToCollect_Structures) false true false false false)))
                (:then_1
                  (bind _asprimaldinocharacter (Utilities|Casting|CastToPrimalDinoCharacter _array_element))
                  (CallFunction|RUTransferAllItems (Variables|/Script/ShooterGame.PrimalCharacter|GetMyInventoryComponent _asprimaldinocharacter) (Variables|Default|GetMyInventoryComponent) (LocalVariables|GetitemsToCollect) false true false false false))))))))))

(fn OnRepIsActivated
  ;[1 1 1] Toggles SFX based on if structure is active
  (Rendering|SetVisibility (Variables|Default|GetParticles) (Variables|Default|GetisActivated) true))

(fn BPContainerDeactivated
  (Variables|Default|SetisActivated false true))