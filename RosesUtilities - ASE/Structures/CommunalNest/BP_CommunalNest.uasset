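; Communal nest structure that auto-collects same-team dropped eggs into its inventory and incubates the fertilized ones.
; Team members toggle fertilized and unfertilized collection through multi-use entries.
; Looping server timers run an octree scan, with radius from the mod's global actor, and drain egg durability scaled by server hatch speed.
; Incubation clamps durability at a floor, and collection skips fertilized eggs near it, so finished eggs are not re-collected.
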(event EventParentFirstBeginPlay
  (Utilities|FlowControl|Sequence
    (:then_0
      ;[1 1 1] Gets auto-collect range config
      (Class|KismetSystemLibrary|IsRunningonServer
        (:Yes
          (bind _globalactor (CallFunction|RUGetGlobalActor self))
          (Variables|Default|SeteffectRange (* 300 (Variables|/Game/Mods/RosesUtilities/RosesUtilities_GlobalActor.RosesUtilities_GlobalActor_C|GetCommunalNestAutoCollectRange _globalactor)) true)
          ;[1 1 1] Gets hatch speed from server config
          (bind _asshootergamestate (Utilities|Casting|CastToShooterGameState (Game|GetGameState)))
          (Variables|Default|SetserverEggHatchSpeedMultiplier (Variables|/Script/ShooterGame.ShooterGameState|GetEggHatchSpeedMultiplier _asshootergamestate)))))
    (:then_1
      ;[1 1 1] Restores saved visibility
      (CallFunction|OnRepEffectRange))
    (:then_2
      ;[1 1 1] Starts collect item scan and incubate eggs loops
      (Class|KismetSystemLibrary|IsRunningonServer
        (:Yes
          (Utilities|FlowControl|Delay 0.5)
          (Utilities|Time|SetTimerbyFunctionName 0 "AutoCollectItems" 1e+01 true)
          (Utilities|FlowControl|Delay 1.0)
          (Utilities|Time|SetTimerbyFunctionName 0 "IncubateEggs" 1e+01 true))))))

(fn ConstructionScript
  (|CallParentFunction))

(fn BPGetMultiUseEntries
  (params (ForPC :type Player%20Controller%20Object%20Reference) (MultiUseEntries :type Array%20of%20Multi%20Use%20Entry%20Structures))
  (bind _returnvalue (|CallParentFunction ForPC MultiUseEntries))
  (LocalVariables|SettempMultiUseEntries _returnvalue)
  (if (== (Variables|Default|GetTargetingTeam) (Variables|/Script/Engine.Actor|GetTargetingTeam ForPC))
    (Utilities|FlowControl|Sequence
      (:then_0
        ;[1 1 1] Adds a MultiUse entry to toggle auto collecting unfertilized eggs on or off
        (Utilities|Array|Add (LocalVariables|GettempMultiUseEntries) (Utilities|Struct|MakeMultiUseEntry 0 (Utilities|String|SelectString "Disable Auto-Collect Unfertilized Eggs" "Enable Auto-Collect Unfertilized Eggs" (Variables|Default|GetisAutoCollectActive_Unfertilized)) 90314 -10000)))
      (:then_1
        ;[1 1 1] Adds a MultiUse entry to toggle auto collecting fertilized eggs on or off
        (Utilities|Array|Add (LocalVariables|GettempMultiUseEntries) (Utilities|Struct|MakeMultiUseEntry 0 (Utilities|String|SelectString "Disable Auto-Collect Fertilized Eggs" "Enable Auto-Collect Fertilized Eggs" (Variables|Default|GetisAutoCollectActive_Fertilized)) 90414 -10001)))
      (:then_2
        (return (LocalVariables|GettempMultiUseEntries))))
    (else
      (return (LocalVariables|GettempMultiUseEntries)))))

(fn BPTryMultiUse
  (params (ForPC :type Player%20Controller%20Object%20Reference) (UseIndex :type Integer))
  (|CallParentFunction ForPC UseIndex)
  (Utilities|FlowControl|Sequence
    (:then_0
      (switch string (Utilities|String|ToString(Integer) UseIndex)
        (:90314
          ;[1 1 1] Toggles unfertilized auto-collect
          (Variables|Default|SetisAutoCollectActive_Unfertilized (not (Variables|Default|GetisAutoCollectActive_Unfertilized)) true))
        (:90414
          ;[1 1 1] Toggles fertilized auto-collect
          (Variables|Default|SetisAutoCollectActive_Fertilized (not (Variables|Default|GetisAutoCollectActive_Fertilized)) true))))
    (:then_1
      (return true))))

(fn AutoCollectItems
  (Class|KismetSystemLibrary|IsRunningonServer
    (:Yes
      ;[1 1 1] Disables if range is 0
      (if (> (Variables|Default|GeteffectRange) 0.0)
        ;[1 1 1] Gets all dropped items in range
        (if (or (Variables|Default|GetisAutoCollectActive_Fertilized) (Variables|Default|GetisAutoCollectActive_Unfertilized))
          (bind _returnvalue (Class|VictoryCore|ServerOctreeOverlapActorsClass (Class|Actor|GetWorld) (Transformation|GetActorLocation) (Variables|Default|GeteffectRange) "ALL_SPATIAL" "/Script/ShooterGame.DroppedItem" true))
          ;[1 1 1] Picks up each dropped egg in range
          (for _array_element _returnvalue
            (if (== (Variables|/Script/Engine.Actor|GetTargetingTeam _array_element) (Variables|Default|GetTargetingTeam))
              (bind _asdroppeditem (Utilities|Casting|CastToDroppedItem _array_element))
              ;[1 1 1] Filters pickup based on if Fertilized or/and Unfertilized should be picked up
              (bind _asprimalitemconsumable_egg_c (Utilities|Casting|CastToPrimalItemConsumable_Egg (Variables|/Script/ShooterGame.DroppedItem|GetMyItem _asdroppeditem)))
              (bind _isfertilized (CallFunction|RUIsEggFertilized _asprimalitemconsumable_egg_c))
              (if (Math|Boolean|ORBoolean (Math|Boolean|ANDBoolean (Variables|Default|GetisAutoCollectActive_Fertilized) (not (Variables|Default|GetisAutoCollectActive_Unfertilized)) _isfertilized) (Math|Boolean|ANDBoolean (not (Variables|Default|GetisAutoCollectActive_Fertilized)) (Variables|Default|GetisAutoCollectActive_Unfertilized) (not _isfertilized)) (and (Variables|Default|GetisAutoCollectActive_Fertilized) (Variables|Default|GetisAutoCollectActive_Unfertilized)))
                ;[1 1 1] Prevents picking up eggs that are done incubating
                (bind _isfertilized_2 (CallFunction|RUIsEggFertilized _asprimalitemconsumable_egg_c))
                (if _isfertilized_2
                  (if (> (Variables|/Script/ShooterGame.PrimalItem|GetItemDurability _asprimalitemconsumable_egg_c) 3.0)
                    (Utilities|FlowControl|Sequence :!label _label
                      (:then_0
                        ;[1 1 1] Stasis check
                        (if (Variables|/Script/Engine.Actor|GetbStasised _asdroppeditem)
                          (Class|Actor|Unstasis _asdroppeditem)))
                      (:then_1
                        ;[1 1 1] Adds egg to inventory and destroys dropped item actor
                        (CallFunction|RUPickupItemtoInventory _asdroppeditem (Variables|Default|GetMyInventoryComponent) (Utilities|Array|MakeArray "/Game/PrimalEarth/CoreBlueprints/Items/Consumables/PrimalItemConsumable_Egg.PrimalItemConsumable_Egg_C")))))
                  (else
                    (goto _label)))))))))))

(fn IncubateEggs
  (Networking|SwitchHasAuthority
    (:Authority
      ;[1 1 1] Gets each fertilized egg to incubate
      (for _array_element (Variables|/Script/ShooterGame.PrimalInventoryComponent|GetInventoryItems (Variables|Default|GetMyInventoryComponent))
        (bind _asprimalitemconsumable_egg_c (Utilities|Casting|CastToPrimalItemConsumable_Egg _array_element))
        (bind _isfertilized (CallFunction|RUIsEggFertilized _asprimalitemconsumable_egg_c))
        (if _isfertilized
          (LocalVariables|SeteggToIncubate _asprimalitemconsumable_egg_c)
          ;[1 1 1] Updates egg incubation
          (Variables|/Script/ShooterGame.PrimalItem|SetItemDurability (LocalVariables|GeteggToIncubate) (Math|Float|Clamp(Float) (- (Variables|/Script/ShooterGame.PrimalItem|GetItemDurability (LocalVariables|GeteggToIncubate)) (* 1e+01 (Variables|/Script/ShooterGame.PrimalItem|GetEggLoseDurabilityPerSecond (LocalVariables|GeteggToIncubate)) (Variables|/Script/ShooterGame.PrimalItem|GetExtraEggLoseDurabilityPerSecondMultiplier (LocalVariables|GeteggToIncubate)) (Variables|Default|GetincubationMultiplier) (Variables|Default|GetserverEggHatchSpeedMultiplier))) 2.0 (Variables|/Script/ShooterGame.PrimalItem|GetItemDurability (LocalVariables|GeteggToIncubate))))
          (Class|PrimalItem|UpdatedItem (LocalVariables|GeteggToIncubate) false))))))